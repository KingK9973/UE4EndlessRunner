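; Endless-runner floor tile that, when its box is overlapped, has RunnerGameMode spawn the next tile, then destroys itself after a short delay.
; Its construction script adds a rock child actor at one of three hindrance points and opens a gap by hiding one of six tiles.
; The gap index is re-rolled to differ from the returned rock index, which is rolled separately from placement.
; GetAttachTransform exposes the Arrow's location for chaining.
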(event OnComponentBeginOverlap(Box)
  (params (OverlappedComponent :type Primitive%20Component%20Object%20Reference) (OtherActor :type Actor%20Object%20Reference) (OtherComp :type Primitive%20Component%20Object%20Reference) (OtherBodyIndex :type Integer) (bFromSweep :type Boolean) (SweepResult :type Hit%20Result%20Structure%20%28by%20ref%29))
  ;[1 1 1] Spawn New Floor And destroy previous one
  (bind _asrunner_game_mode (Utilities|Casting|CastToRunnerGameMode (Game|GetGameMode)))
  (Default|SpawnFloorTile _asrunner_game_mode false)
  (Utilities|FlowControl|Delay 2.0)
  (Actor|DestroyActor))

(event EventBeginPlay)

(event Collision|EventActorBeginOverlap
  (params (OtherActor :type Actor%20Object%20Reference)))

(event EventTick
  (params (DeltaSeconds :type Float%20%28single-precision%29)))

(fn ConstructionScript
  (if (not (Variables|Default|GetINITIAL))
    (Utilities|FlowControl|DoOnce false
      (:Completed
        (CallFunction|SetRockHindrancePoint)
        (CallFunction|SetTileHindranceLocations)
        (bind _returnvalue (CallFunction|RockHindranceBlocker))
        (CallFunction|TileHindranceBlocker _returnvalue)))))

(fn GetAttachTransform
  (return (Math|Transform|MakeTransform (.Location (Math|Transform|BreakTransform (Transformation|GetWorldTransform (Variables|Default|GetArrow)))))))

(fn SetRockHindrancePoint
  (Variables|Default|SetRockHindrancePonts (Utilities|Array|MakeArray (Math|Conversions|ToTransform(Vector) (Variables|/Script/Engine.SceneComponent|GetRelativeLocation (Variables|Default|GetHindrance1))) (Math|Conversions|ToTransform(Vector) (Variables|/Script/Engine.SceneComponent|GetRelativeLocation (Variables|Default|GetHindrance2))) (Math|Conversions|ToTransform(Vector) (Variables|/Script/Engine.SceneComponent|GetRelativeLocation (Variables|Default|GetHindrance3)))))
  (return))

(fn RockHindranceBlocker
  (bind _rockhindranceponts (Variables|Default|GetRockHindrancePonts))
  (bind _returnvalue (Utilities|Array|LastIndex _rockhindranceponts))
  (bind _returnvalue_2 (Math|Random|RandomIntegerinRange 0 _returnvalue))
  (AddComponent|AddChildActorComponent false (Utilities|Array|Get(acopy) _rockhindranceponts _returnvalue_2))
  (return _returnvalue_2))

(fn SetTileHindranceLocations
  (Variables|Default|SetTilesHindrancePoint (Utilities|Array|MakeArray (Variables|Default|GetTile1) (Variables|Default|GetTile2) (Variables|Default|GetTile3) (Variables|Default|GetTile4) (Variables|Default|GetTile5) (Variables|Default|GetTile6)))
  (return))

(fn TileHindranceBlocker
  (params (rockLoc :type Integer))
  (LocalVariables|SetNewLocalVar_1 rockLoc)
  (bind _asrunner_game_mode (Utilities|Casting|CastToRunnerGameMode (Game|GetGameMode)))
  (bind _randomnumber (Default|Random _asrunner_game_mode :!label _label))
  (LocalVariables|SetNewLocalVar_2 _randomnumber)
  (if (== (LocalVariables|GetNewLocalVar_1) (LocalVariables|GetNewLocalVar_2))
    (goto _label)
    (else
      (LocalVariables|SetNewLocalVar_0 (Utilities|Array|Get(acopy) (Variables|Default|GetTilesHindrancePoint) (LocalVariables|GetNewLocalVar_2)))
      (Collision|SetCollisionEnabled (LocalVariables|GetNewLocalVar_0) "NoCollision")
      (Rendering|SetVisibility (LocalVariables|GetNewLocalVar_0) false false))))