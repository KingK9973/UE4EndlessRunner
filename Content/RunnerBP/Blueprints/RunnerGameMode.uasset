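; Game mode for a runner game that lays the track by spawning floor tiles end to end.
; BeginPlay spawns a starting batch flagged as initial, with SpawnFloorTile storing each tile's attach transform as the next spawn point.
; A separate Random function, not called here, returns a deterministic stepped number that climbs and falls within a small range, using a direction flag and alternating decrements.
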(event EventBeginPlay
  (for _index (range 0 3)
    (CallFunction|SpawnFloorTile true)))

(fn ConstructionScript)

(fn SpawnFloorTile
  (params (INITIAL :type Boolean))
  (bind _returnvalue (Game|SpawnActorfromClass "/Game/RunnerBP/Blueprints/FloorTile.FloorTile_C" (Variables|Default|GetNewVar_0) "Undefined" 0 INITIAL 0))
  (bind _attchtransform (Default|GetAttachTransform _returnvalue))
  (Variables|Default|SetNewVar_0 _attchtransform))

(fn Random
  (bind _output_get (Variables|Default|SetRandomNumber (+ (Variables|Default|GetRandomNumber) (Variables|Default|Getinc))))
  (if (Variables|Default|Getflag)
    (if (>= (+ (Variables|Default|GetConvert1) _output_get) 0)
      (Variables|Default|Setinc (Variables|Default|GetConvert1))
      (if (== (Variables|Default|GetConvert1) -4) :!label _label
        (Variables|Default|SetConvert1 -2)
        (else
          (Variables|Default|SetConvert1 -4)))
      (return (Variables|Default|GetRandomNumber))
      (elif (<= (+ (Variables|Default|GetConvert1) _output_get) 0)
        (Variables|Default|Setflag false)
        (goto _label)))
    (elif (<= (+ _output_get 3) 5)
      (Variables|Default|Setinc 3)
      (if (>= (+ _output_get 2) 5) :!label _label_2
        (Variables|Default|Setflag true :!label _label_3)
        (Variables|Default|Setinc 0)
        (return (Variables|Default|GetRandomNumber)))
      (elif (<= (+ _output_get 2) 5)
        (Variables|Default|Setinc 2)
        (goto _label_2)
        (else
          (goto _label_3))))))